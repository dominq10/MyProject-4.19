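; Scripted-motion Blueprint for a skeletal mesh, named as a tongue, that moves along a timeline and triggers another Blueprint.
; BeginPlay stops the mesh animation, then Tick calls Play on the timeline every frame.
; Timeline tracks set world location and yaw, and feed integer switches that gate non-looping animation playback.
; A further track value opens the referenced ddaw_Blueprint2, so one timeline sequences movement, animation and the trigger.
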(event `self.ReceiveBeginPlay`
  (`SkeletalMeshComponent.Stop` (`self.SkeletalMeshComponent`)))

(event `self.ReceiveTick`
  (params (DeltaSeconds :type "Float (single-precision)"))
  (bind (_direction _123 _1234 _newtrack_3 _newtrack_0) (`Timeline|Timeline_0`)
    (:`Update`
      (`SceneComponent.K2_SetWorldLocationAndRotation` (`self.SkeletalMeshComponent`) _newtrack_0 (`KismetMathLibrary.MakeRotator` 0.0 0.0 _123) false false)
      (switch `int` (`KismetMathLibrary.FTrunc` _1234)
        (:`Default`
          (`SkeletalMeshComponent.Play` (`self.SkeletalMeshComponent`) false)
          (switch `int` (`KismetMathLibrary.FTrunc` _newtrack_3)
            (:`1`
              (bind _asddaw_blueprint_2 (cast `/Game/ddaw_Blueprint2` (`self.NewVar_0`)))
              (`/Game/ddaw_Blueprint2.open` _asddaw_blueprint_2))))))))

(fn `UserConstructionScript`)