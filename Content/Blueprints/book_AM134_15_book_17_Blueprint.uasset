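; Interactive book prop that works as a two-step trigger, advanced each time its Itter event fires.
; The first call hides the mesh and moves it to a hardcoded world position and rotation.
; The second shows it there and calls Upal on two referenced cube actors, cast to 1313_Blueprint and Cube19_Blueprint.
; The Inv counter tracks the step, and later calls do nothing.
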(event `/Game/Blueprints/112233.itter`
  (bind _staticmeshcomponent (`self.StaticMeshComponent`))
  (switch `int` (`self.inv`)
    (:`0`
      (set `self.inv` 1)
      (`SceneComponent.SetVisibility` _staticmeshcomponent false false)
      (`SceneComponent.K2_SetWorldLocationAndRotation` (`self.StaticMeshComponent`) (-465.0 -1100.0 751.0) (struct :`Pitch` 271.0) false false))
    (:`1`
      (set `self.inv` 2)
      (`SceneComponent.SetVisibility` _staticmeshcomponent true false)
      (bind _as1313_blueprint (cast `/Game/Blueprints/1313_Blueprint` (`self.cube1`)))
      (`/Game/Blueprints/1313_Blueprint.upal` _as1313_blueprint)
      (bind _ascube_19_blueprint (cast `/Game/Blueprints/Cube19_Blueprint` (`self.cube`)))
      (`/Game/Blueprints/Cube19_Blueprint.upal` _ascube_19_blueprint))))

(fn `UserConstructionScript`)