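; Inspectable-object actor that toggles its mesh in front of the player's camera for viewing and rotation.
; An externally callable event flip-flops between saving the mesh location, placing it ahead of the camera with Gaussian depth-of-field, and changing the blur settings while sending it to world origin.
; Box overlap enables or disables input, letting Turn and LookUp axes accumulate into mesh roll and pitch.
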(event `CustomEvent_1`
  (`SceneComponent.K2_SetWorldRotation` (`self.StaticMeshComponent`) (`KismetMathLibrary.MakeRotator` (stale `InputAxis|Turn` _output_get) (* (stale `InputAxis|LookUp` _output_get) -1.0)) false false :!label _label))

(event `InputAxis|Turn`
  (params (AxisValue :type "Float (single-precision)"))
  (bind _output_get (set `self.X` (+ (`self.X`) AxisValue)))
  (goto _label))

(event `InputAxis|LookUp`
  (params (AxisValue :type "Float (single-precision)"))
  (bind _output_get (set `self.y` (+ (`self.y`) AxisValue)))
  (goto _label))

(event `CustomEvent`
  (bind _aschar (cast `/Game/char` (`GameplayStatics.GetPlayerCharacter` 0)))
  (bind _camera (`/Game/char.Camera` _aschar))
  (bind _output_get (set `/Game/char.Camera` _camera _aschar))
  (`/Engine/EditorBlueprintResources/StandardMacros.FlipFlop`
    (:`A`
      (bind _output_get_2 (set `self.Position Zhyr` (`SceneComponent.K2_GetComponentLocation` (`self.StaticMeshComponent`))))
      (set `CameraComponent.PostProcessSettings` (make `PostProcessSettings` :`DepthOfFieldMethod` "DOFM_Gaussian" :`DepthOfFieldFstop` 7.0 :`DepthOfFieldFocalDistance` 220.0 :`DepthOfFieldDepthBlurRadius` 1.0 :`DepthOfFieldNearTransitionRegion` 966.0 :`DepthOfFieldFarTransitionRegion` 0.0 :`DepthOfFieldScale` 1.0 :`DepthOfFieldFarBlurSize` 23.0) _camera)
      (`SceneComponent.K2_SetWorldLocation` (`self.StaticMeshComponent`) (+ (* (`SceneComponent.GetForwardVector` _output_get) 150) (`SceneComponent.K2_GetComponentLocation` _output_get)) false false))
    (:`B`
      (set `self.Position Zhyr` _output_get_2)
      (set `CameraComponent.PostProcessSettings` (make `PostProcessSettings` :`DepthOfFieldMethod` "DOFM_Gaussian" :`DepthOfFieldFstop` 7.0 :`DepthOfFieldFocalDistance` 220.0 :`DepthOfFieldDepthBlurRadius` 1.0 :`DepthOfFieldFocalRegion` 10000.0 :`DepthOfFieldNearTransitionRegion` 966.0 :`DepthOfFieldFarTransitionRegion` 0.0 :`DepthOfFieldScale` 1.0 :`DepthOfFieldFarBlurSize` 23.0) _output_get)
      (`SceneComponent.K2_SetWorldLocation` (`self.StaticMeshComponent`) (0.0 0.0 0.0) false false))))

(event `self.Box.OnComponentBeginOverlap`
  (params (OverlappedComponent :type "PrimitiveComponent Object Reference") (OtherActor :type "Actor Object Reference") (OtherComp :type "PrimitiveComponent Object Reference") (OtherBodyIndex :type Integer) (bFromSweep :type Boolean) (SweepResult :type "HitResult Structure (by ref)"))
  (`self.EnableInput` (`GameplayStatics.GetPlayerController` 0)))

(event `self.Box.OnComponentEndOverlap`
  (params (OverlappedComponent :type "PrimitiveComponent Object Reference") (OtherActor :type "Actor Object Reference") (OtherComp :type "PrimitiveComponent Object Reference") (OtherBodyIndex :type Integer))
  (`self.DisableInput` (`GameplayStatics.GetPlayerController` 0)))

(fn `UserConstructionScript`)