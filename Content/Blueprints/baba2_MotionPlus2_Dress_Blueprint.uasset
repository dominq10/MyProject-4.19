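; Blueprint for a dress skeletal mesh, apparently a motion variant, whose visibility and animation playback are driven by a timeline.
; BeginPlay hides the mesh and stops its animation, and Tick keeps calling Play on the timeline.
; Each timeline update truncates the track value to set visibility, then switches on it, with the default branch playing the animation without looping.
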(event `self.ReceiveBeginPlay`
  (`SceneComponent.SetVisibility` (`self.SkeletalMeshComponent`) false false)
  (`SkeletalMeshComponent.Stop` (`self.SkeletalMeshComponent`)))

(event `self.ReceiveTick`
  (params (DeltaSeconds :type "Float (single-precision)"))
  (bind (_direction _newtrack_0) (`Timeline|Timeline_0`)
    (:`Update`
      (bind _returnvalue (`KismetMathLibrary.FTrunc` _newtrack_0))
      (`SceneComponent.SetVisibility` (`self.SkeletalMeshComponent`) (`KismetMathLibrary.Conv_IntToBool` _returnvalue) false)
      (switch `int` _returnvalue
        (:`Default`
          (`SkeletalMeshComponent.Play` (`self.SkeletalMeshComponent`) false))))))

(fn `UserConstructionScript`)